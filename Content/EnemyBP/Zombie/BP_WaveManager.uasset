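; BP_WaveManager spawns waves of BP_ZombieEnemy pawns running BT_Zombie at random actors tagged ZombieSpawn.
; StartWave stores count and speed, then SpawnSingleZombie re-calls itself after a short delay until the count is used up, setting each walk speed.
; StartNextRound destroys existing zombies and, inside that same loop, starts a wave sized from the round number with increased speed, so it fires only if zombies exist, once per zombie.
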(event Custom|StartWave
  (params (Count :type Integer) (Speed :type Integer))
  ;[0.15 0.15 0.15 0.5] ZombieSpawner
  (Actor|GetAllActorswithTag "ZombieSpawn")
  (bind _output_get (Variables|Default|SetZombiesToSpawn Count))
  (Variables|Default|SetZombiesRemainingAlive _output_get)
  (Variables|Default|SetSpeedForRound (Math|Conversions|ToFloat(Integer) Speed))
  (CallFunction|SpawnSingleZombie))

(event Custom|SpawnSingleZombie
  ;[0.15 0.15 0.15 0.5] ZombieSpawner
  (if (> (Variables|Default|GetZombiesToSpawn) 0)
    (bind _outactors (Actor|GetAllActorswithTag "ZombieSpawn"))
    (bind _returnvalue (AI|SpawnAIFromClass "/Game/EnemyBP/Zombie/BP_ZombieEnemy.BP_ZombieEnemy_C" "/Game/EnemyBP/Zombie/BT_Zombie.BT_Zombie" (.location (Transformation|GetActorTransform (Utilities|Array|Get(acopy) _outactors (Math|Random|RandomIntegerinRange 0 (Utilities|Array|LastIndex _outactors))))) (.rotation (Transformation|GetActorTransform (Utilities|Array|Get(acopy) _outactors (Math|Random|RandomIntegerinRange 0 (Utilities|Array|LastIndex _outactors))))) true 0))
    (bind _ascharacter (Utilities|Casting|CastToCharacter _returnvalue))
    (Variables|/Script/Engine.CharacterMovementComponent|SetMaxWalkSpeed (Variables|/Script/Engine.Character|GetCharacterMovement _ascharacter) (Variables|Default|GetSpeedForRound))
    (Variables|Default|SetZombiesToSpawn (- (Variables|Default|GetZombiesToSpawn) 1))
    (if (> (Variables|Default|GetZombiesToSpawn) 0)
      (Utilities|FlowControl|Delay 0.01)
      (CallFunction|SpawnSingleZombie))))

(event Custom|StartNextRound
  (params (IncomingRoundNumber :type Boolean))
  ;[0.15 0.15 0.15 0.5] ZombieSpawner
  (bind _outactors (Actor|GetAllActorsOfClass "/Game/EnemyBP/Zombie/BP_ZombieEnemy.BP_ZombieEnemy_C"))
  (for _array_element _outactors
    (Actor|DestroyActor _array_element)
    (Variables|Default|SetCurrentRound (Math|Conversions|ToInteger(Boolean) IncomingRoundNumber))
    (bind _output_get (Variables|Default|SetZombiesToSpawn (* IncomingRoundNumber 2)))
    (CallFunction|StartWave _output_get (Math|Float|Truncate (+ (Variables|Default|GetSpeedForRound) 2e+01)))))

(event EventBeginPlay)

(event Collision|EventActorBeginOverlap
  (params (OtherActor :type Actor%20Object%20Reference)))

(event EventTick
  (params (DeltaSeconds :type Float%20%28single-precision%29)))

(fn ConstructionScript)