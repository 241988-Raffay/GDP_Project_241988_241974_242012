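; Zombie enemy that melees the first-person player and dies when its health runs out.
; Taking damage sets the damage causer as the AI blackboard's TargetActor; death detaches the controller, stops movement, plays animation and sound, then freezes the mesh.
; Attackzone overlap starts a looping timer for delayed-hit attacks; leaving clears it and restores the Animation Blueprint.
; An AIMoveTo chase loop is left unconnected, and GetDeathStatus exposes the dead flag.
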(event OnComponentBeginOverlap(Attackzone)
  (params (OverlappedComponent :type Primitive%20Component%20Object%20Reference) (OtherActor :type Actor%20Object%20Reference) (OtherComp :type Primitive%20Component%20Object%20Reference) (OtherBodyIndex :type Integer) (bFromSweep :type Boolean) (SweepResult :type Hit%20Result%20Structure%20%28by%20ref%29))
  ;[0.15 0.15 0.15 0.5] PlayerDamage
  (if (not (Variables|Default|GetIsDead))
    (bind _asbp_first_person_character (Utilities|Casting|CastToBP_FirstPersonCharacter OtherActor))
    (bind _output_get (Variables|Default|SetTargetPlayer _asbp_first_person_character))
    (CallFunction|DoDamage)
    (bind _returnvalue (Utilities|Time|SetTimerbyEvent (delegate Custom|DoDamage) 2.0 true))
    (bind _output_get_2 (Variables|Default|SetAttackTime _returnvalue))))

(event OnComponentEndOverlap(Attackzone)
  (params (OverlappedComponent :type Primitive%20Component%20Object%20Reference) (OtherActor :type Actor%20Object%20Reference) (OtherComp :type Primitive%20Component%20Object%20Reference) (OtherBodyIndex :type Integer))
  ;[0.15 0.15 0.15 0.5] PlayerDamage
  (Utilities|Time|ClearandInvalidateTimerbyHandle (stale OnComponentBeginOverlap(Attackzone) _output_get_2))
  (Utilities|FlowControl|Delay 1.0)
  (Components|Animation|SetAnimationMode (Variables|Character|GetMesh) "AnimationBlueprint" true))

(event Custom|DoDamage
  ;[0.15 0.15 0.15 0.5] PlayerDamage
  (Components|Animation|PlayAnimation (Variables|Character|GetMesh) "/Game/EnemyBP/Zombie/source/Zombie_Anim_attack.Zombie_Anim_attack" false)
  (Audio|PlaySoundatLocation "/Game/EnemyBP/Zombie/SFX/Zombie_attack.Zombie_attack" (Transformation|GetActorLocation) "0, 0, 0" 1.0 1.0 0.0 0 0 0 0)
  (Utilities|FlowControl|Delay 0.5)
  (Game|Damage|ApplyDamage (stale OnComponentBeginOverlap(Attackzone) _output_get) 15.0 0 0))

(event EventBeginPlay
  ;[0.15 0.15 0.15 0.5] Follow Character
)

(event Game|Damage|EventAnyDamage
  (params (Damage :type Float%20%28single-precision%29) (DamageType :type Damage%20Type%20Object%20Reference) (InstigatedBy :type Controller%20Object%20Reference) (DamageCauser :type Actor%20Object%20Reference))
  (bind _asaicontroller (Utilities|Casting|CastToAIController (Pawn|GetController))
    (:then
      (AI|Components|Blackboard|SetValueasObject (AI|GetBlackboard _asaicontroller) (Utilities|Name|MakeLiteralName "TargetActor") DamageCauser))
    (:CastFailed
      _))
  (Variables|Default|SetHealth (- (Variables|Default|GetHealth) Damage))
  (if (<= (Variables|Default|GetHealth) 0.0)
    (Utilities|FlowControl|DoOnce false
      (:Completed
        (Variables|Default|SetIsDead true)
        (Components|Movement|StopMovementImmediately (Variables|Character|GetCharacterMovement))
        (Pawn|Components|CharacterMovement|SetMovementMode (Variables|Character|GetCharacterMovement) "MOVE_None" 0)
        (Class|Pawn|DetachfromControllerPendingDestroy)
        (Components|Animation|PlayAnimation (Variables|Character|GetMesh) "/Game/EnemyBP/Zombie/source/Zombie_Anim_death.Zombie_Anim_death" false)
        (Transformation|AddActorLocalOffset "0.000000,0.000000,-10.000000" false false)
        (Audio|PlaySoundatLocation "/Game/EnemyBP/Zombie/SFX/death3.death3" (Transformation|GetActorLocation) "0, 0, 0" 1.0 1.0 0.0 0 0 0 0)
        (Collision|SetCollisionEnabled (Variables|Character|GetMesh) "NoCollision")
        (Variables|Default|SetbUseControllerRotationYaw false)
        (Utilities|FlowControl|Delay 1.77)
        (Components|Tick|SetComponentTickEnabled (Variables|Character|GetMesh) false)))))

(fn ConstructionScript)

(fn GetDeathStatus
  (return (Variables|Default|GetIsDead)))