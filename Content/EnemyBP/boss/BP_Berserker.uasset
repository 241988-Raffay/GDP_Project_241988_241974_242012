(event OnComponentBeginOverlap(Sphere)
  (params (OverlappedComponent :type Primitive%20Component%20Object%20Reference) (OtherActor :type Actor%20Object%20Reference) (OtherComp :type Primitive%20Component%20Object%20Reference) (OtherBodyIndex :type Integer) (bFromSweep :type Boolean) (SweepResult :type Hit%20Result%20Structure%20%28by%20ref%29))
  ;[0.15 0.15 0.15 0.5] Attack Anims
  (Utilities|Casting|CastToBP_FirstPersonCharacter OtherActor)
  (switch int (Math|Random|RandomIntegerinRange 0 2)
    (:0
      (Animation|PlayAnimMontage "/Game/EnemyBP/boss/slendytubbies-iii-skintubbyberserker/source/AM_Attack1.AM_Attack1" 1.0 "None"))
    (:1
      (Animation|PlayAnimMontage "/Game/EnemyBP/boss/slendytubbies-iii-skintubbyberserker/source/AM_Attack2.AM_Attack2" 1.0 "None"))
    (:2
      (Animation|PlayAnimMontage "/Game/EnemyBP/boss/slendytubbies-iii-skintubbyberserker/source/AM_Attack3.AM_Attack3" 1.0 "None"))))

(event Custom|ExecuteSummon
  ;[0.15 0.15 0.15 0.5] Summon Ability
  (Game|SpawnActorfromClass "/Game/EnemyBP/Zombie/BP_ZombieEnemy.BP_ZombieEnemy_C" (Transformation|GetActorTransform (Variables|Default|GetSpawn1)) "Undefined" "MultiplyWithRoot" 0 0)
  (Game|SpawnActorfromClass "/Game/EnemyBP/Zombie/BP_ZombieEnemy.BP_ZombieEnemy_C" (Transformation|GetActorTransform (Variables|Default|GetSpawn2)) "Undefined" "MultiplyWithRoot" 0 0)
  (Game|SpawnActorfromClass "/Game/EnemyBP/BurntZombie/BP_ZombieBurnt.BP_ZombieBurnt_C" (Transformation|GetActorTransform (Variables|Default|GetSpawn3)) "Undefined" "MultiplyWithRoot" 0 0)
  (Game|SpawnActorfromClass "/Game/EnemyBP/BurntZombie/BP_ZombieBurnt.BP_ZombieBurnt_C" (Transformation|GetActorTransform (Variables|Default|GetSpawn4)) "Undefined" "MultiplyWithRoot" 0 0))

(event EventBeginPlay
  ;[0.15 0.15 0.15 0.5] Set Health
  (Default|SetHealthStartingValues (Variables|Default|GetBPC_health)))

(event Collision|EventActorBeginOverlap
  (params (OtherActor :type Actor%20Object%20Reference)))

(event EventTick
  (params (DeltaSeconds :type Float%20%28single-precision%29))
  (bind _returnvalue (Game|GetPlayerCharacter 0))
  (bind _charactermovement (Variables|Character|GetCharacterMovement))
  (bind _returnvalue_2 (Transformation|GetDistanceTo _returnvalue))
  ;[0.15 0.15 0.15 0.5] Boss Runs to Player if Player is far away from Boss
  (if (< _returnvalue_2 4e+02)
    (Variables|/Script/Engine.CharacterMovementComponent|SetMaxWalkSpeed _charactermovement 1.8e+02)
    (Variables|Default|SetbIsSprinting false)
    (AI|AIMoveTo self (Transformation|GetActorLocation (Game|GetPlayerCharacter 0)) 0 1.5e+02 false :!label _label)
    (elif (> _returnvalue_2 1e+03)
      (Variables|/Script/Engine.CharacterMovementComponent|SetMaxWalkSpeed _charactermovement 6.5e+02)
      (Variables|Default|SetbIsSprinting true)
      (goto _label))))

(fn ConstructionScript)