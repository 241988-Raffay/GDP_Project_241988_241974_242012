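; BP_ZombieEnemy is a zombie enemy character that takes damage and dies.
; AnyDamage lowers Health; at zero it stops movement and rotation, then once sets IsDead, plays a random death sound and disables movement and mesh collision.
; GetDeathStatus exposes IsDead.
; A looping AIMoveTo chase of the player exists but is unconnected, as BeginPlay does nothing, so it never runs.
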(event EventBeginPlay
  ;[0.15 0.15 0.15 0.5] Follow Character
)

(event Game|Damage|EventAnyDamage
  (params (Damage :type Float%20%28single-precision%29) (DamageType :type Damage%20Type%20Object%20Reference) (InstigatedBy :type Controller%20Object%20Reference) (DamageCauser :type Actor%20Object%20Reference))
  ;[0.15 0.15 0.15 0.5] Damage and Death
  (Variables|Default|SetHealth (- (Variables|Default|GetHealth) Damage))
  (if (<= (Variables|Default|GetHealth) 0.0)
    (bind _output_get (Variables|/Script/Engine.CharacterMovementComponent|SetbOrientRotationToMovement (Variables|Character|GetCharacterMovement) false))
    (Variables|Default|SetbUseControllerRotationYaw _output_get)
    (Components|Movement|StopMovementImmediately (Variables|Character|GetCharacterMovement))
    (Utilities|FlowControl|DoOnce false
      (:Completed
        (Variables|Default|SetIsDead true)
        (Audio|SpawnSoundatLocation (.OutItem (Utilities|Array|Random (Variables|Default|GetDeathSounds))) (Transformation|GetActorLocation) "0, 0, 0" 1.0 1.0 0.0 "/Game/EnemyBP/terror-engine-male-zombie/SFX/NewSoundAttenuation.NewSoundAttenuation" 0)
        (Pawn|Components|CharacterMovement|DisableMovement (Variables|Character|GetCharacterMovement))
        (Collision|SetCollisionEnabled (Variables|Character|GetMesh) "NoCollision")))))

(fn ConstructionScript)

(fn GetDeathStatus
  (return (Variables|Default|GetIsDead)))