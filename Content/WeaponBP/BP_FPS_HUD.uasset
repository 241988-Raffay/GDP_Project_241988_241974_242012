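; First-person HUD Blueprint that draws a crosshair while the player carries a handgun.
; Each DrawHUD casts the player character to BP_FirstPersonCharacter and checks its HasHandgun flag.
; When the flag is set, it draws the M_Crosshair material as a small fixed-size square at the screen center.
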(event EventDrawHUD
  (params (SizeX :type Integer) (SizeY :type Integer))
  ;[0.15 0.15 0.15 0.5] Draw CrosshairHUD
  ;[0.15 0.15 0.15 0.5] Only draws HUD when player has Handgun
  (bind _asbp_first_person_character (Utilities|Casting|CastToBP_FirstPersonCharacter (Game|GetPlayerCharacter 0)))
  (if (Variables|/Game/FirstPerson/Blueprints/BP_FirstPersonCharacter.BP_FirstPersonCharacter_C|GetHasHandgun _asbp_first_person_character)
    (Canvas|DrawMaterial "/Game/Textures/M_Crosshair.M_Crosshair" (- (Math|Conversions|ToFloat(Integer) (/ SizeX 2)) 4.0) (- (Math|Conversions|ToFloat(Integer) (/ SizeY 2)) 4.0) 8.0 8.0 0.0 0.0 0.0)))

(fn ConstructionScript)